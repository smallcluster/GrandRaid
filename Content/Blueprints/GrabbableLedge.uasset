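; GrabbableLedge is a climbable ledge that shows its Key prompt while the PlayerCharacter overlaps it.
; It enables input for player controller 0 and, on the action press, checks that the player is inside its Box.
; It projects the player's location onto the ledge's yaw-based right-vector line, passes that point, the actor rotation and Edge's height to StartClimbing, then hides the prompt.
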(event `self.ReceiveBeginPlay`
  (`self.EnableInput` (`GameplayStatics.GetPlayerController` 0))
  (`SceneComponent.SetVisibility` (`self.key`) false false))

(event `self.ReceiveActorBeginOverlap`
  (params (OtherActor :type "Actor Object Reference"))
  (cast `/Game/Blueprints/PlayerCharacter` OtherActor)
  (`SceneComponent.SetVisibility` (`self.key`) true false))

(event `self.ReceiveActorEndOverlap`
  (params (OtherActor :type "Actor Object Reference"))
  (cast `/Game/Blueprints/PlayerCharacter` OtherActor)
  (`SceneComponent.SetVisibility` (`self.key`) false false))

(event `InputAction|action` :consume false
  (params (Key :type "Key Structure"))
  (bind _returnvalue (`GameplayStatics.GetPlayerCharacter` 0))
  (bind _returnvalue_2 (`self.K2_GetActorLocation`))
  (bind (_returnvalue_roll _returnvalue_pitch _returnvalue_yaw) (`KismetMathLibrary.BreakRotator` (`self.K2_GetActorRotation`)))
  (bind (_returnvalue_x _returnvalue_y _returnvalue_z) (`KismetMathLibrary.BreakVector` (`SceneComponent.K2_GetComponentLocation` (`self.edge`))))
  (bind _returnvalue_3 (`KismetMathLibrary.Normal` (`KismetMathLibrary.GetRightVector` (`KismetMathLibrary.MakeRotator` 0.0 0.0 _returnvalue_yaw))))
  (:`Pressed`
    (if (`PrimitiveComponent.IsOverlappingActor` (`self.Box`) _returnvalue)
      (bind _asplayer_character (cast `/Game/Blueprints/PlayerCharacter` _returnvalue))
      (`/Game/Blueprints/PlayerCharacter.startClimbing` _asplayer_character (`self.K2_GetActorRotation`) (+ (* _returnvalue_3 (`KismetMathLibrary.Dot_VectorVector` _returnvalue_3 (- (`self.K2_GetActorLocation` _returnvalue) _returnvalue_2))) _returnvalue_2) _returnvalue_z)
      (`SceneComponent.SetVisibility` (`self.key`) false false))))

(fn `UserConstructionScript`)