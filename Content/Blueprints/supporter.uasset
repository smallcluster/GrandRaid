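; Crowd supporter actor that shows a randomly chosen animated character.
; On BeginPlay it picks a random mesh and one of that mesh's animations from Data, then plays it looped from a random start time so supporters vary.
; Each Tick it toggles mesh visibility by squared distance to the player character, or to the IntroCamera pawn when that cast fails, as a simple distance cull.
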(event `self.ReceiveBeginPlay`
  (bind _anim (`self.anim`))
  (bind _skeletalmesh (`self.SkeletalMesh`))
  (bind _output_get (set `self.skinAndAnims` (`KismetArrayLibrary.Array_Random` (`self.data`))))
  (set `self.Mesh` (break `/Game/Blueprints/supporterData` _output_get))
  (set `self.anim` (`KismetArrayLibrary.Array_Random` (`.animations_8_B8D7E7EC4D45ADAAD818CBAFE75119A2` (break `/Game/Blueprints/supporterData` _output_get))))
  (`SkinnedMeshComponent.SetSkinnedAssetAndUpdate` _skeletalmesh (`self.Mesh`) true)
  (`SkeletalMeshComponent.SetAnimation` _skeletalmesh _anim)
  (`SkeletalMeshComponent.SetPosition` _skeletalmesh (`KismetMathLibrary.RandomFloatInRange` 0.0 (`AnimSequenceBase.SequenceLength` _anim)) false)
  (`SkeletalMeshComponent.Play` _skeletalmesh true))

(event `self.ReceiveTick`
  (params (DeltaSeconds :type "Float (single-precision)"))
  (bind _skeletalmesh (`self.SkeletalMesh`))
  (bind _asplayer_character (cast `/Game/Blueprints/PlayerCharacter` (`GameplayStatics.GetPlayerCharacter` 0))
    (:`then`
      (if (< (`KismetMathLibrary.Vector_DistanceSquared` (`self.K2_GetActorLocation` _asplayer_character) (`self.K2_GetActorLocation`)) 16000000.0)
        (`SceneComponent.SetVisibility` _skeletalmesh true false :!label _label)
        (else
          (`SceneComponent.SetVisibility` _skeletalmesh false false :!label _label_2))))
    (:`CastFailed`
      (bind _asintro_camera (cast `/Game/Blueprints/IntroCamera` (`GameplayStatics.GetPlayerPawn` 0)))
      (if (< (`KismetMathLibrary.Vector_DistanceSquared` (`self.K2_GetActorLocation` _asintro_camera) (`self.K2_GetActorLocation`)) 16000000.0)
        (goto _label)
        (else
          (goto _label_2))))))

(fn `UserConstructionScript`)