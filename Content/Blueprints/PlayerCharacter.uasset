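; Player character with axis-driven movement and look, a climbing action, a toggleable spotlight and a disable flag that blocks movement.
; StartClimbing, when not falling, aligns actor and mesh and flags the PlayerABP; EndClimbing resets the mesh and teleports the actor to the pelvis socket at the stored height plus an offset.
; Tick pins the spring arm and spotlight to pelvis and head sockets, so they follow the animated mesh.
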(event `self.ReceiveBeginPlay`
  (`SceneComponent.SetVisibility` (`self.SpotLight`) false false))

(event `InputAction|action`
  (params (Key :type "Key Structure")))

(event `InputAxis|MoveForward`
  (params (AxisValue :type "Float (single-precision)"))
  (bind (_returnvalue_roll _returnvalue_pitch _returnvalue_yaw) (`KismetMathLibrary.BreakRotator` (`self.GetControlRotation`)))
  ;[1 1 1] Movement
  (if (`self.disable`)
    _
    (elif (not (`self.isClimbing`))
      (`self.AddMovementInput` (`KismetMathLibrary.GetForwardVector` (`KismetMathLibrary.MakeRotator` 0.0 0.0 _returnvalue_yaw)) AxisValue))))

(event `InputAxis|MoveRight`
  (params (AxisValue :type "Float (single-precision)"))
  (bind (_returnvalue_roll _returnvalue_pitch _returnvalue_yaw) (`KismetMathLibrary.BreakRotator` (`self.GetControlRotation`)))
  ;[1 1 1] Movement
  (if (`self.disable`)
    _
    (elif (not (`self.isClimbing`))
      (`self.AddMovementInput` (`KismetMathLibrary.GetRightVector` (`KismetMathLibrary.MakeRotator` 0.0 0.0 _returnvalue_yaw)) AxisValue))))

(event `InputAxis|lookingUp`
  (params (AxisValue :type "Float (single-precision)"))
  (`self.AddControllerPitchInput` AxisValue))

(event `InputAxis|Turn`
  (params (AxisValue :type "Float (single-precision)"))
  (`self.AddControllerYawInput` AxisValue))

(event `self.ReceiveTick`
  (params (DeltaSeconds :type "Float (single-precision)"))
  (`SceneComponent.K2_SetWorldLocation` (`self.SpringArm`) (`SceneComponent.GetSocketLocation` (`self.Mesh`) "pelvisSocket") false false)
  (`SceneComponent.K2_SetWorldLocation` (`self.SpotLight`) (`SceneComponent.GetSocketLocation` (`self.Mesh`) "headSocket") false false))

(fn `disablePlayer`
  (set `self.disable` true))

(fn `EndClimbing`
  (bind (_returnvalue_x _returnvalue_y) (`KismetMathLibrary.BreakVector` (`SceneComponent.GetSocketLocation` (`self.Mesh`) "pelvisSocket")))
  (`SceneComponent.K2_SetRelativeLocation` (`self.Mesh`) (0.0 0.0 -85.0) false false)
  (`self.K2_TeleportTo` (`KismetMathLibrary.MakeVector` _returnvalue_x _returnvalue_y (+ (`self.Z`) 88.0)) (`self.K2_GetActorRotation`))
  (set `self.isClimbing` false))

(fn `hideLight`
  (`SceneComponent.SetVisibility` (`self.SpotLight`) false false))

(fn `showLight`
  (`SceneComponent.SetVisibility` (`self.SpotLight`) true false))

(fn `startClimbing`
  (params (rotation :type "Rotator Structure") (meshPos :type "Vector Structure") (Z :type "Float (double-precision)"))
  (bind _mesh (`self.Mesh`))
  (bind (_returnvalue_x _returnvalue_y _returnvalue_z) (`KismetMathLibrary.BreakVector` (`SceneComponent.K2_GetComponentLocation` _mesh)))
  (bind _asplayer_abp (cast `/Game/Blueprints/PlayerABP` (`SkeletalMeshComponent.GetAnimInstance` (`self.Mesh`))))
  (if (not (`/Game/Blueprints/PlayerABP.isFalling` _asplayer_abp))
    (if (not (`self.isClimbing`))
      (bind _asplayer_abp_2 (cast `/Game/Blueprints/PlayerABP` (`SkeletalMeshComponent.GetAnimInstance` (`self.Mesh`))))
      (set `self.Z` Z)
      (`self.K2_SetActorRotation` rotation)
      (`SceneComponent.K2_SetWorldLocation` _mesh (`KismetMathLibrary.MakeVector` meshPos_X meshPos_Y _returnvalue_z) false false)
      (set `/Game/Blueprints/PlayerABP.isClimbing` true _asplayer_abp_2)
      (set `self.isClimbing` true))))

(fn `UserConstructionScript`)