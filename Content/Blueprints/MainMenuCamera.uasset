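; Main menu camera actor that travels along a spline while staying aimed at a target component.
; Each tick, Move advances a distance by speed and delta time, wraps it at the spline length for a continuous loop, and places the camera at that point in world space.
; LookAt then rotates the camera to face the target's world location.
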(event `self.ReceiveTick`
  (params (DeltaSeconds :type "Float (single-precision)"))
  (`self.move` DeltaSeconds)
  (`self.lookAt`))

(fn `lookAt`
  (`SceneComponent.K2_SetWorldRotation` (`self.Camera`) (`KismetMathLibrary.FindLookAtRotation` (`SceneComponent.K2_GetComponentLocation` (`self.Camera`)) (`SceneComponent.K2_GetComponentLocation` (`self.target`))) false false))

(fn `move`
  (params (`delta time` :type "Float (double-precision)"))
  (bind _output_get (set `self.dist` (mod (+ (`self.dist`) (* (`self.speed`) `delta time`)) (`SplineComponent.GetSplineLength` (`self.Spline`)))))
  (`SceneComponent.K2_SetWorldLocation` (`self.Camera`) (`SplineComponent.GetLocationAtDistanceAlongSpline` (`self.Spline`) _output_get "World") false false))

(fn `UserConstructionScript`)