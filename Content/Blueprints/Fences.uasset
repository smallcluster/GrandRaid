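; Fence actor that lays fence segments along an editable spline, built entirely in the Construction Script.
; The spline length divided by FenceLength sets the segment count, and each segment is a spline mesh component with query and physics collision.
; Each segment spans consecutive distances along the spline on the X forward axis, with tangents clamped to FenceLength.
; The event graph holds no logic.
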(fn `UserConstructionScript`
  (bind _spline (`self.Spline`))
  (bind _spline_2 (`self.Spline`))
  (bind _spline_3 (`self.Spline`))
  (`SplineComponent.SetSplinePointType` (`self.Spline`) (`SplineComponent.GetNumberOfSplinePoints` _spline_2) "Linear" true)
  (for _index (range (+ (`KismetMathLibrary.FTrunc` (/ (`SplineComponent.GetSplineLength` _spline_2) (`self.fenceLength`))) 1))
    (bind _returnvalue (`AddComponent|NODE_AddSplineMeshComponent-0`))
    (`PrimitiveComponent.SetCollisionEnabled` _returnvalue "QueryAndPhysics")
    (`SplineMeshComponent.SetForwardAxis` _returnvalue "X" true)
    (bind _returnvalue_2 (* _index (`self.fenceLength`)))
    (bind _returnvalue_3 (* (+ _index 1) (`self.fenceLength`)))
    (`SplineMeshComponent.SetStartAndEnd` _returnvalue (`SplineComponent.GetLocationAtDistanceAlongSpline` _spline_3 _returnvalue_2 "Local") (`KismetMathLibrary.ClampVectorSize` (`SplineComponent.GetTangentAtDistanceAlongSpline` _spline_3 _returnvalue_2 "Local") 0.0 (`self.fenceLength`)) (`SplineComponent.GetLocationAtDistanceAlongSpline` _spline _returnvalue_3 "Local") (`KismetMathLibrary.ClampVectorSize` (`SplineComponent.GetTangentAtDistanceAlongSpline` _spline _returnvalue_3 "Local") 0.0 (`self.fenceLength`)) true)))